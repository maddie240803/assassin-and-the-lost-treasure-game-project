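; Player-controlled assassin character for a side-scroller, with movement along X, jumping, sword attacks, health and death handling.
; Enhanced Input drives movement, blocked while attacking, and attacks that branch into ground or airborne versions, each spawning a momentary Attack actor.
; DoOnce gates with separate reset events throttle attacks.
; Death respawns at the start location, while Death_2 shows the game-over widget; both play the death animation state.
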(event Custom|Death
  ;[1 1 1] Death
  (Input|DisableInput 0)
  (Class|PaperZDAnimInstance|JumptoNode (Variables|/Script/PaperZD.PaperZDAnimationComponent|GetAnimInstance (Variables|Default|GetAnimationComponent)) "death" "None")
  (Utilities|FlowControl|Delay 0.7)
  (Transformation|SetActorLocation (Variables|Default|GetSpawn) false false)
  (Components|Activation|SetActive (Variables|Character|GetCharacterMovement) true false)
  (Input|EnableInput 0))

(event Custom|ResetAttack
  ;[1 1 1] Attack and Jump
  (Utilities|FlowControl|DoOnce false) ; enters at Reset
)

(event Custom|Death_2
  (Input|DisableInput 0)
  (Class|PaperZDAnimInstance|JumptoNode (Variables|/Script/PaperZD.PaperZDAnimationComponent|GetAnimInstance (Variables|Default|GetAnimationComponent)) "death" "None")
  (Utilities|FlowControl|Delay 0.7)
  (bind _returnvalue (UserInterface|CreateWidget "/Game/Game_over.Game_over_C"))
  (UserInterface|Viewport|AddtoViewport _returnvalue 0)
  (bind _asbp_assassin (Utilities|Casting|CastToBP_assassin (Game|GetPlayerCharacter 0)))
  (Variables|/Script/Engine.PlayerController|SetbShowMouseCursor (Game|GetPlayerController (Variables|/Script/Engine.Pawn|GetPlayerState _asbp_assassin)) true))

(event Custom|ResetIdleAttack
  ;[1 1 1] Attack and Jump
  (Utilities|FlowControl|DoOnce false) ; enters at Reset
)

(event Custom|ResetJumpAttack
  ;[1 1 1] Attack and Jump
  (Utilities|FlowControl|DoOnce false) ; enters at Reset
)

(event Input|EnhancedActionEvents|EnhancedInputActionIA_move
  (params (ActionValue :type Vector%202D%20Structure) (ElapsedSeconds :type Float%20%28double-precision%29) (TriggeredSeconds :type Float%20%28double-precision%29) (InputAction :type Input%20Action%20Object%20Reference :default "/Game/assassin/IA_move.IA_move"))
  ;[1 1 1] Movement
  (if (not (Variables|Default|Getattack))
    (Pawn|Input|AddMovementInput "2.000000,0.000000,0.000000" (.x ActionValue) false)
    (Pawn|SetControlRotation (Pawn|GetController) (select (> (.x ActionValue) 0.0) (Math|Rotator|MakeRotator 0.0 0.0 0.0) (Math|Rotator|MakeRotator 0.0 0.0 1.8e+02)))))

(event Input|EnhancedActionEvents|EnhancedInputActionIA_attack
  (params (ActionValue :type Boolean) (ElapsedSeconds :type Float%20%28double-precision%29) (TriggeredSeconds :type Float%20%28double-precision%29) (InputAction :type Input%20Action%20Object%20Reference :default "/Game/assassin/IA_attack.IA_attack"))
  ;[1 1 1] Attack and Jump
  (Utilities|FlowControl|DoOnce false
    (:Completed
      (Variables|Default|Setattack true)
      (if (not (AI|Components|NavMovement|IsFalling (Variables|Character|GetCharacterMovement)))
        (Utilities|FlowControl|DoOnce false
          (:Completed
            (Variables|Default|SetIdleAttack true)
            ;[1 1 1] Hit
            (Audio|PlaySound2D "/Game/Audio/sword-sound-260274__mp3cut_net_.sword-sound-260274__mp3cut_net_" 1.0 1.0 0.0 0 0)
            (bind _returnvalue (Game|SpawnActorfromClass "/Game/RedSamurai/attack.attack_C" (Transformation|GetWorldTransform (Variables|Default|GetScene)) "Undefined" "MultiplyWithRoot" 0 0))
            (Actor|DestroyActor _returnvalue)))
        (else
          (Utilities|FlowControl|DoOnce false
            (:Completed
              (Variables|Default|Setjumpattack true)
              (Audio|PlaySound2D "/Game/Audio/sword-sound-260274__mp3cut_net_.sword-sound-260274__mp3cut_net_" 1.0 1.0 0.0 0 0)
              (bind _returnvalue_2 (Game|SpawnActorfromClass "/Game/RedSamurai/attack.attack_C" (Transformation|GetWorldTransform (Variables|Default|GetScene)) "Undefined" "MultiplyWithRoot" 0 0))
              (Actor|DestroyActor _returnvalue_2))))))))

(event EventBeginPlay
  (Variables|Default|SetSpawn (Transformation|GetActorLocation))
  (bind _asplayer_controller (Utilities|Casting|CastToPlayerController (Pawn|GetController)))
  (Utilities|IsValid (PlayerController|LocalPlayerSubsystems|GetEnhancedInputLocalPlayerSubsystem _asplayer_controller)
    (:Is%20Valid
      (Input|AddMappingContext (PlayerController|LocalPlayerSubsystems|GetEnhancedInputLocalPlayerSubsystem _asplayer_controller) "/Game/assassin/assassin_InputMappingContext.assassin_InputMappingContext" 0 "(bIgnoreAllPressedKeysUntilRelease=True,bForceImmediately=False,bNotifyUserSettings=False)"))))

(event Game|Damage|EventAnyDamage
  (params (Damage :type Float%20%28single-precision%29) (DamageType :type Damage%20Type%20Object%20Reference) (InstigatedBy :type Controller%20Object%20Reference) (DamageCauser :type Actor%20Object%20Reference))
  ;[1 1 1] Damage
  (Variables|Default|SetHealth (- (Variables|Default|GetHealth) Damage))
  (if (<= (Variables|Default|GetHealth) 0.0)
    (CallFunction|Death2)))

(event Input|KeyboardEvents|SpaceBar
  (params (Key :type Key%20Structure :default "None"))
  (:Pressed
    (Audio|PlaySound2D "/Game/Audio/lightattack4.lightattack4" 1.0 1.0 0.0 0 0)
    (Character|Jump))
  (:Released
    (Character|StopJumping)))

(fn ConstructionScript)