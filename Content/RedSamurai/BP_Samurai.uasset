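; Samurai enemy with flipbook animation that walks forward, flips around whenever an overlap with its Box ends, and attacks the player.
; The Hit volume switches run and attack flipbooks; while the player overlaps it, Tick stops movement and repeats a delayed forward sphere trace.
; Trace hits damage BP_assassin and trigger its Death at zero health.
; Incoming damage is scaled by 100, updates the BP_Enemy health widget, and destroys the samurai at zero.
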(event OnComponentEndOverlap(Box)
  (params (OverlappedComponent :type Primitive%20Component%20Object%20Reference) (OtherActor :type Actor%20Object%20Reference) (OtherComp :type Primitive%20Component%20Object%20Reference) (OtherBodyIndex :type Integer))
  ;[1 1 1] Player turning
  (Transformation|SetActorRotation (Math|Rotator|CombineRotators (Transformation|GetActorRotation) "0.000000,180.000000,0.000000")))

(event OnComponentBeginOverlap(hit)
  (params (OverlappedComponent :type Primitive%20Component%20Object%20Reference) (OtherActor :type Actor%20Object%20Reference) (OtherComp :type Primitive%20Component%20Object%20Reference) (OtherBodyIndex :type Integer) (bFromSweep :type Boolean) (SweepResult :type Hit%20Result%20Structure%20%28by%20ref%29))
  ;[1 1 1] player detector
  (Utilities|Casting|CastToBP_assassin OtherActor)
  (Sprite|SetFlipbook (Variables|Default|GetSprite) "/Game/RedSamurai/Spritesheet/sheets/Samurai_atk/Samurai_atk.Samurai_atk"))

(event OnComponentEndOverlap(hit)
  (params (OverlappedComponent :type Primitive%20Component%20Object%20Reference) (OtherActor :type Actor%20Object%20Reference) (OtherComp :type Primitive%20Component%20Object%20Reference) (OtherBodyIndex :type Integer))
  ;[1 1 1] player detector
  (Utilities|Casting|CastToBP_assassin OtherActor)
  (Sprite|SetFlipbook (Variables|Default|GetSprite) "/Game/RedSamurai/Spritesheet/sheets/Samurai_run/Samurai_run.Samurai_run"))

(event EventTick
  (params (DeltaSeconds :type Float%20%28single-precision%29))
  ;[1 1 1] MoveMent and Enemy attack hit
  (if (Collision|IsOverlappingActor (Variables|Default|Gethit) (Game|GetPlayerCharacter 0) :!class /Script/Engine.PrimitiveComponent)
    (Utilities|FlowControl|DoOnce false :!label _label
      (:Completed
        (Utilities|FlowControl|RetriggerableDelay 0.5)
        (CallFunction|AttackTrace)
        (goto _label Reset)))
    (else
      (bind _asbp_assassin (Utilities|Casting|CastToBP_assassin (Game|GetPlayerCharacter 0)))
      (Variables|Default|SetAs%20BP%20Assassin _asbp_assassin)
      (Pawn|Input|AddMovementInput (Transformation|GetActorForwardVector) 0.3 false))))

(event EventBeginPlay
  ;[1 1 1] Current Health
  (bind _asbp_enemy (Utilities|Casting|CastToBP_Enemy (UserInterface|GetUserWidgetObject (Variables|Default|GetWidget))))
  (Variables|Default|SetAs%20BP%20Enemy_0 _asbp_enemy)
  (Variables|/Game/RedSamurai/BP_Enemy.BP_Enemy_C|SetCurrentHealth _asbp_enemy (Variables|Default|GetCurrentHealth))
  (Variables|/Game/RedSamurai/BP_Enemy.BP_Enemy_C|SetMaxHealth _asbp_enemy (Variables|Default|GetMaxHealth)))

(event Game|Damage|EventAnyDamage
  (params (Damage :type Float%20%28single-precision%29) (DamageType :type Damage%20Type%20Object%20Reference) (InstigatedBy :type Controller%20Object%20Reference) (DamageCauser :type Actor%20Object%20Reference))
  ;[1 1 1] apply Enemy damage
  (bind _output_get (Variables|Default|SetCurrentHealth (- (Variables|Default|GetCurrentHealth) (* Damage 1e+02))))
  (Default|Healing (Variables|Default|GetAs%20BP%20Enemy_0) _output_get)
  (if (<= (Variables|Default|GetCurrentHealth) 0.0)
    (Actor|DestroyActor)))

(fn ConstructionScript)

(fn AttackTrace
  (bind _returnvalue (Transformation|GetActorLocation))
  (bind _outhit (Collision|SphereTraceForObjects _returnvalue (+ _returnvalue (* (Transformation|GetActorForwardVector) 2.5e+02)) 0.0 (Utilities|Array|MakeArray "ObjectTypeQuery3") false 0 "None"))
  (bind _asbp_assassin (Utilities|Casting|CastToBP_assassin (.HitActor (Collision|BreakHitResult _outhit))))
  (Game|Damage|ApplyDamage _asbp_assassin 25.0 0 0)
  (if (<= (Variables|/Game/assassin/BP_assassin.BP_assassin_C|GetHealth (Variables|Default|GetAs%20BP%20Assassin)) 0.0)
    (Default|Death (Variables|Default|GetAs%20BP%20Assassin))))